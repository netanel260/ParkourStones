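; Player Blueprint that lets the player interact with objects or drag physics bodies the camera is pointed at.
; A per-tick camera line trace looks for BPI_Interact actors or simulating components, toggling an "Interact"/"Drag" prompt widget and a gate on the input.
; Pressing Interact sends the interface message and grabs the hit component with a Physics Handle, whose target follows the trace's end point until release.
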(event `InputAction|Interact`
  (params (Key :type "Key Structure"))
  (bind _hitcomponenttrace (`self.HitComponentTrace`))
  (:`Pressed`
    (`/Engine/EditorBlueprintResources/StandardMacros.Gate` true :!label _label
      (:`Exit`
        (message `/Game/_Blueprints/BPI_Interact.Interact` (`.HitActor` (`GameplayStatics.BreakHitResult` (stale `self.ReceiveTick` _outhit))))
        (`PhysicsHandleComponent.GrabComponentAtLocation` (`self.PhysicsHandle`) _hitcomponenttrace "None" (`SceneComponent.K2_GetComponentLocation` _hitcomponenttrace)))))
  (:`Released`
    (`PhysicsHandleComponent.ReleaseComponent` (`self.PhysicsHandle`))))

(event `self.ReceiveTick`
  (params (DeltaSeconds :type "Float (single-precision)"))
  (bind _returnvalue (`GameplayStatics.GetPlayerCameraManager` 0))
  (bind _returnvalue_2 (`PlayerCameraManager.GetCameraLocation` _returnvalue))
  (bind _returnvalue_3 (+ _returnvalue_2 (* (`self.GetActorForwardVector` _returnvalue) 250.0)))
  (`|ExecutionSequence`
    (:`then_0`
      (bind (_outhit _returnvalue_4) (`KismetSystemLibrary.LineTraceSingle` :`Start` _returnvalue_2 :`End` _returnvalue_3 :`TraceChannel` "TraceTypeQuery1" :`DrawDebugType` "ForOneFrame"))
      (if _returnvalue_4
        (bind (_bblockinghit _binitialoverlap _time _distance _location _impactpoint _normal _impactnormal _physmat _hitactor _hitcomponent) (`GameplayStatics.BreakHitResult` _outhit))
        (bind _output_get (set `self.InteractActor` _hitactor))
        (set `self.HitComponentTrace` _hitcomponent)
        (if (or (`KismetSystemLibrary.DoesImplementInterface` _output_get "/Game/_Blueprints/BPI_Interact.BPI_Interact_C") (`SceneComponent.IsSimulatingPhysics` _hitcomponent "None"))
          (`/Engine/EditorBlueprintResources/StandardMacros.DoOnce` false :!label _label_2
            (:`Completed`
              (`Widget.SetVisibility` (`self.InteractionWidget`) "Visible")
              (set `/Game/_UI/WBP_InteractPrompt.InteractionTypeText` (select `bool` (`SceneComponent.IsSimulatingPhysics` (`self.HitComponentTrace`) "None") :`false` "Interact" :`true` "Drag" :!type "Text") (`self.InteractionWidget`))
              (goto _label :!via `Open`)))
          (else
            _))
        (else
          (set `self.InteractActor` null)
          (set `self.HitComponentTrace` null)))
      (`|ExecutionSequence`
        (:`then_0`
          (goto _label_2 :!via `Reset`))
        (:`then_1`
          (`Widget.SetVisibility` (`self.InteractionWidget`) "Hidden")
          (goto _label :!via `Close`))))
    (:`then_1`
      (`PhysicsHandleComponent.SetTargetLocation` (`self.PhysicsHandle`) _returnvalue_3))))

(event `self.ReceiveBeginPlay`
  (bind _returnvalue (`|CreateWidget` "/Game/_UI/WBP_InteractPrompt.WBP_InteractPrompt_C"))
  (bind _output_get (set `self.InteractionWidget` _returnvalue))
  (`UserWidget.AddToViewport` _output_get 0)
  (`Widget.SetVisibility` (`self.InteractionWidget`) "Hidden"))

(fn `UserConstructionScript`)