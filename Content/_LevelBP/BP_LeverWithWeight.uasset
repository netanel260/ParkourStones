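; BP_LeverWithWeight is a one-shot interactable lever that drops its handle and triggers a linked actor.
; Interact, gated by CanUseHandle, calls MoveHandleDown, which eases HandleRoot through a quarter-turn roll and calls CallLeverDown.
; If the linked Actor is valid, it runs a named custom function via a short timer, activates the actor's components and sends InteractMessage.
; HandleDown is never cleared here, so the lever does not return.
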(event `MoveHandleDown`
  (bind _actor (`self.Actor`))
  (bind _handleroot (`self.HandleRoot`))
  (bind (_preveousrot_roll _preveousrot_pitch _preveousrot_yaw) (`KismetMathLibrary.BreakRotator` (`self.PreveousRot`)))
  (if (not (`self.HandleDown`))
    (set `self.HandleDown` true)
    (set `self.PreveousRot` (`SceneComponent.RelativeRotation` _handleroot))
    (`KismetSystemLibrary.MoveComponentTo` _handleroot (0.0 0.0 0.0) (`KismetMathLibrary.MakeRotator` (+ _preveousrot_roll 90.0) _preveousrot_pitch _preveousrot_yaw) true false 1.0)
    (`self.LeverDown` true)
    (`/Engine/EditorBlueprintResources/StandardMacros.IsValid` _actor
      (:`Is Valid`
        (`KismetSystemLibrary.K2_SetTimer` _actor (`self.ActorCustomFunction`) 0.1)
        (for _array_element (`self.K2_GetComponentsByClass` (`self.Actor`) "/Script/Engine.ActorComponent")
          (`ActorComponent.Activate` _array_element false))
        (message `/Game/_Blueprints/BPI_Interact.Interact` (`self.Actor`))))))

(event `/Game/_Blueprints/BPI_Interact.Interact`
  (if (`self.CanUseHandle`)
    (`self.MoveHandleDown`)))

(fn `UserConstructionScript`)