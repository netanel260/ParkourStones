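; Pressure plate that unlocks a linked lever while a physics-simulating object rests on it.
; When such a component enters the sphere trigger, the plate sinks with a sound and sets CanUseHandle on the referenced LeverActor.
; When it leaves, the plate rises back with another sound and the lever's handle is disabled again.
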(event `self.Sphere.OnComponentBeginOverlap`
  (params (OverlappedComponent :type "PrimitiveComponent Object Reference") (OtherActor :type "Actor Object Reference") (OtherComp :type "PrimitiveComponent Object Reference") (OtherBodyIndex :type Integer) (bFromSweep :type Boolean) (SweepResult :type "HitResult Structure (by ref)"))
  (if (`SceneComponent.IsSimulatingPhysics` OtherComp "None")
    (`GameplayStatics.PlaySound2D` "/Game/_Sounds/pressure-plate-45634.pressure-plate-45634" 1.0 1.0 0.0 null null)
    (`KismetSystemLibrary.MoveComponentTo` (`self.PresurePlate`) (0.0 0.0 -10.0) (struct) false false 1.0)
    (set `/Game/_LevelBP/BP_LeverWithWeight.CanUseHandle` true (`self.LeverActor`))))

(event `self.Sphere.OnComponentEndOverlap`
  (params (OverlappedComponent :type "PrimitiveComponent Object Reference") (OtherActor :type "Actor Object Reference") (OtherComp :type "PrimitiveComponent Object Reference") (OtherBodyIndex :type Integer))
  (if (`SceneComponent.IsSimulatingPhysics` OtherComp "None")
    (`GameplayStatics.PlaySound2D` "/Game/_Sounds/bow-release-bow-and-arrow-4-101936.bow-release-bow-and-arrow-4-101936" 1.0 1.0 0.0 null null)
    (`KismetSystemLibrary.MoveComponentTo` (`self.PresurePlate`) (0.0 0.0 0.0) (struct) false false 1.0)
    (set `/Game/_LevelBP/BP_LeverWithWeight.CanUseHandle` false (`self.LeverActor`))))

(fn `UserConstructionScript`)